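; Startup actor that stages a character preview and opens the character selection screen.
; BeginPlay stores a self reference and spawns BP_MainCharacter at an offset from its mesh, keeping that reference for the selection widget.
; LoadSelectionScreen shows W_CharacterSelection with the mouse cursor and adds one labeled button per entry in the supplied slots array.
; Key 1 prints controller ID, username and slot values from Admin.csv in the server save directory, apparently for debugging.
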(event EventBeginPlay
  ;[1 1 1] Spawn Character
  (Variables|Default|SetBP_StartupCharacterViewRef self)
  (bind _returnvalue (Game|SpawnActorfromClass "/Game/Startup/Characters/BP_MainCharacter.BP_MainCharacter_C" (Math|Transform|MakeTransform (+ (Transformation|GetWorldLocation (Variables|Character|GetMesh)) "450.000000,50.000000,75.000000") "0,160.000000, 0") "AlwaysSpawn" 0 0))
  (Variables|Default|SetBP_MainCharacterRef _returnvalue))

(event Input|KeyboardEvents|1
  (params (Key :type Key%20Structure :default "None"))
  (:Pressed
    (bind (_stringarray _returnvalue) (Class|TextFileManager|LoadArrayText (Utilities|String|Append (Utilities|Struct|BreakDirectoryPath (Variables|Default|GetServer%20Save%20Directory)) "/Admin.csv")))
    (if _returnvalue
      (for _array_element (Utilities|Array|MakeArray (Utilities|String|Append "Controller ID: " (Utilities|Array|Get(acopy) _stringarray 1)) (Utilities|String|Append "Username: " (Utilities|Array|Get(acopy) _stringarray 2)) (Utilities|String|Append "Slot1:" (Utilities|Array|Get(acopy) _stringarray 3)) (Utilities|String|Append "Slot2:" (Utilities|Array|Get(acopy) _stringarray 4)) (Utilities|String|Append "Slot3:" (Utilities|Array|Get(acopy) _stringarray 5)) (Utilities|String|Append "Slot4" (Utilities|Array|Get(acopy) _stringarray 6)))
        (Development|PrintString _array_element))
      (else
        (Development|PrintString "Hello")))))

(fn ConstructionScript)

(fn LoadSelectionScreen
  (params (PlayerName :type String) (Player :type Player%20Controller%20Object%20Reference) (SlotsArray :type Array%20of%20Strings))
  (Variables|Default|SetPlayer%20Name PlayerName)
  (Variables|Default|SetPlayer Player)
  (LocalVariables|SetLocalSlotsArray SlotsArray)
  (bind _returnvalue (UserInterface|CreateWidget "/Game/Startup/Widgets/W_CharacterSelection.W_CharacterSelection_C" 0 (Variables|Default|GetBP_MainCharacterRef)))
  (UserInterface|Viewport|AddtoViewport _returnvalue 0)
  (Variables|/Script/Engine.PlayerController|SetbShowMouseCursor (Variables|Default|GetPlayer) true)
  (for _array_element (LocalVariables|GetLocalSlotsArray)
    (bind _returnvalue_2 (UserInterface|CreateWidget "/Game/Startup/Widgets/W_CharacterSelectionButtons.W_CharacterSelectionButtons_C" (Variables|Default|GetPlayer)))
    (Rendering|Components|TextRender|SetText (Variables|/Game/Startup/Widgets/W_CharacterSelectionButtons.W_CharacterSelectionButtons_C|GetCharacterChoiceText _returnvalue_2) (Utilities|Text|ToText(String) _array_element))
    (Default|AddCharacterButton _returnvalue _returnvalue_2)))