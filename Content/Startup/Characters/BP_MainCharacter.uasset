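; BP_MainCharacter is the player character, with camera-relative movement, look, jump and sprint.
; Jump and sprint apply locally and also call SER events that repeat the action, apparently server RPCs, with sprint switching max walk speed.
; The construction script picks a male or female mannequin mesh from IsMale, both sharing one AnimBP.
; It also provides a MoveToMap level-open helper and a debug Escape-to-quit key.
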(event Custom|SER_StopSprint
  ;[1 1 1] Jump / Sprint
  (Variables|/Script/Engine.CharacterMovementComponent|SetMaxWalkSpeed (Variables|Character|GetCharacterMovement) 6e+02))

(event Custom|SER_Sprint
  ;[1 1 1] Jump / Sprint
  (Variables|/Script/Engine.CharacterMovementComponent|SetMaxWalkSpeed (Variables|Character|GetCharacterMovement) 1e+03))

(event Custom|SER_Jump
  ;[1 1 1] Jump / Sprint
  (Character|Jump))

(event Custom|SER_StopJump
  ;[1 1 1] Jump / Sprint
  (Character|StopJumping))

(event Input|ActionEvents|InputActionJump
  (params (Key :type Key%20Structure :default "None"))
  ;[1 1 1] Jump / Sprint
  (:Pressed
    (CallFunction|SERJump)
    (Character|Jump))
  (:Released
    (CallFunction|SERStopJump)
    (Character|StopJumping)))

(event Input|ActionEvents|InputActionSprint
  (params (Key :type Key%20Structure :default "None"))
  (bind _charactermovement (Variables|Character|GetCharacterMovement))
  ;[1 1 1] Jump / Sprint
  (:Pressed
    (CallFunction|SERSprint)
    (Variables|/Script/Engine.CharacterMovementComponent|SetMaxWalkSpeed _charactermovement 1e+03))
  (:Released
    (CallFunction|SERStopSprint)
    (Variables|/Script/Engine.CharacterMovementComponent|SetMaxWalkSpeed _charactermovement 6e+02)))

(event Input|AxisEvents|InputAxisMoveForward
  (params (AxisValue :type Float%20%28single-precision%29))
  ;[1 1 1] Movement
  (Pawn|Input|AddMovementInput (Math|Vector|GetForwardVector (Math|Rotator|MakeRotator 0.0 0.0 (.Yaw (Math|Rotator|BreakRotator (Pawn|GetControlRotation :!class /Script/Engine.Pawn))))) AxisValue false))

(event Input|AxisEvents|InputAxisMoveRight
  (params (AxisValue :type Float%20%28single-precision%29))
  ;[1 1 1] Movement
  (Pawn|Input|AddMovementInput (Math|Vector|GetRightVector (Math|Rotator|MakeRotator 0.0 0.0 (.Yaw (Math|Rotator|BreakRotator (Pawn|GetControlRotation :!class /Script/Engine.Pawn))))) AxisValue false))

(event Input|AxisEvents|InputAxisLookUp
  (params (AxisValue :type Float%20%28single-precision%29))
  ;[1 1 1] Movement
  (Pawn|Input|AddControllerPitchInput AxisValue))

(event Input|AxisEvents|InputAxisTurn
  (params (AxisValue :type Float%20%28single-precision%29))
  ;[1 1 1] Movement
  (Pawn|Input|AddControllerYawInput AxisValue))

(event Input|KeyboardEvents|Escape
  (params (Key :type Key%20Structure :default "None"))
  ;[1 1 1] Debug Quit Game
  (:Pressed
    (bind _asmain_player_controller (Utilities|Casting|CastToMainPlayerController (Pawn|GetController self)))
    (Game|QuitGame _asmain_player_controller "Quit" false)))

(fn ConstructionScript
  (bind _mesh (Variables|Character|GetMesh))
  (bind _mesh_2 (Variables|Character|GetMesh))
  (if (Variables|Default|GetIsMale)
    (Class|SkinnedMeshComponent|SetSkeletalMesh _mesh_2 "/Game/Mannequin/Character/Mesh/SK_Mannequin.SK_Mannequin" true)
    (Class|SkeletalMeshComponent|SetAnimClass _mesh_2 "/Game/Mannequin/Animations/ThirdPerson_AnimBP.ThirdPerson_AnimBP_C")
    (Variables|Default|SetIsMale true)
    (else
      (Class|SkinnedMeshComponent|SetSkeletalMesh _mesh "/Game/Mannequin/Character/Mesh/SK_Mannequin_Female.SK_Mannequin_Female" true)
      (Class|SkeletalMeshComponent|SetAnimClass _mesh "/Game/Mannequin/Animations/ThirdPerson_AnimBP.ThirdPerson_AnimBP_C")
      (Variables|Default|SetIsMale false))))

(fn MovetoMap
  (params (Map :type Name))
  (Game|OpenLevel(byName) Map))