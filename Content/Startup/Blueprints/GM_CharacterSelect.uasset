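; Game mode for the login and character selection screen, handling user accounts, character creation and entry to Map01.
; Login only checks that the user's CSV exists, then spawns a viewer, preview character and slot buttons; passwords go unchecked.
; Creation validates the name, writes character and inventory CSVs, records one of four user slots, then possesses the character.
; Loading an existing character is unfinished, only checking its file before moving to the map.
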(event Custom|LoginAttemptSent
  (params (Username :type Text) (Password :type Text) (LoginWidgetRef :type W%20Login%20Screen%20Object%20Reference))
  ;[1 1 1] Login registered user
  (Networking|SwitchHasAuthority
    (:Authority
      (Variables|Names|SetUsername Username)
      (Variables|References|SetNewPlayerLoginWidget LoginWidgetRef)
      (bind _fileexists (CallFunction|FindSaveFile "CSV" (Utilities|String|ToString(Text) (Variables|Names|GetUsername))))
      (if _fileexists
        ;[1 1 1] Get data and fill character selection widget
        (bind _slotsarray (CallFunction|LoadCharacterSelection self (Variables|References|GetNewPlayer) (Variables|Names|GetUsername)))
        (Variables|CharacterSots|SetSlots%20Array _slotsarray)
        ;[1 1 1] Spawn StartupCharacterViewer
        (bind _success (CallFunction|CreateStartupCharacterViewer (Variables|References|GetNewPlayer)))
        (if _success
          ;[1 1 1] Create Character Selection Screen Widget
          (CallFunction|CreateCharacterSelectionScreenWidget (Variables|CharacterSots|GetSlots%20Array))
          ;[1 1 1] Close login widget
          (Widget|RemovefromParent (Variables|References|GetNewPlayerLoginWidget))
          ;[1 1 1] Create MainCharacter in view of StartupCharacterViewer
          (bind _success_2 (CallFunction|SpawnMainCharacterinSelectionScreen (Variables|References|GetBP_StartupCharacterViewer)))
          (if (not _success_2)
            (Development|PrintString "Failed to spawn MainCharacter in Selection Screen!"))
          (else
            (Development|PrintString "Failed to spawn StartupCharacterViewer")))
        (else
          (Development|PrintString "User file doesn't exist." true true "(R=0.000000,G=0.660000,B=1.000000,A=1.000000)" 1e+01))))))

(event Custom|CreateNewUser
  (params (Username :type Text) (Password :type Text) (LoginWidgetRef :type W%20Login%20Screen%20Object%20Reference))
  ;[1 1 1] Create a new user
  (bind _success (CallFunction|GetNewUser Username Password LoginWidgetRef))
  (if _success
    (bind _slotsarray (CallFunction|LoadCharacterSelection self (Variables|References|GetNewPlayer) (Variables|Names|GetUsername)))
    (Variables|CharacterSots|SetSlots%20Array _slotsarray)
    ;[1 1 1] Spawn StartupCharacterViewer
    (bind _success_2 (CallFunction|CreateStartupCharacterViewer (Variables|References|GetNewPlayer)))
    (if _success_2
      ;[1 1 1] Create Character Selection Widget
      (CallFunction|CreateCharacterSelectionScreenWidget (Variables|CharacterSots|GetSlots%20Array))
      ;[1 1 1] Close Login Widget
      (Widget|RemovefromParent (Variables|References|GetNewPlayerLoginWidget))
      ;[1 1 1] Create MainCharacter in view of StartupCharacterViewer
      (bind _success_3 (CallFunction|SpawnMainCharacterinSelectionScreen (Variables|References|GetBP_StartupCharacterViewer)))
      (if _success_3
        (Development|PrintString "spawned MainCharacter" true true "(R=0.000000,G=0.660000,B=1.000000,A=1.000000)" 6.0)
        (else
          (Development|PrintString "Failed to spawn MainCharacter in Selection Screen!")))
      (else
        (Development|PrintString "Failed to spawn StartupCharacterViewer")))
    (else
      (Development|PrintString "Failed to make save file."))))

(event Custom|CreateCharacter
  (params (CharacterName :type String) (IsMale :type Boolean))
  ;[1 1 1] Create new character and spawn on starter location
  (bind _success (CallFunction|CreateNewCharacter CharacterName IsMale))
  (if _success
    (CallFunction|LoadPlayerHUD)
    (Default|MovetoMap (Variables|References|GetMain%20Character%20Ref) "Map01")))

(event Custom|LoadCharacter
  (params (CharacterName :type String))
  ;[1 0.3749 0.6205] Load Character and spawn at saved location
  (CallFunction|LoadSelectedPlayer CharacterName)
  (CallFunction|LoadPlayerHUD)
  (Default|MovetoMap (Variables|References|GetMain%20Character%20Ref) "Map01"))

(event EventPostLogin
  (params (NewPlayer :type Player%20Controller%20Object%20Reference))
  ;[1 1 1] On Player Login
  (bind _output_get (Variables|References|SetNewPlayer NewPlayer))
  (CallFunction|CreateLoginWidget _output_get))

(fn ConstructionScript)

(fn CreateNewCharacter
  (params (CharacterName :type String) (IsMale :type Boolean))
  ;[1 1 1] Check if character already exists.
  (LocalVariables|SetLocalCharacterName CharacterName)
  (LocalVariables|SetLocalIsMale IsMale)
  (bind _infile (CallFunction|CheckCharacterExists (LocalVariables|GetLocalCharacterName)))
  (if _infile
    (Development|PrintString "Character name already exists.")
    (return false)
    (else
      ;[1 1 1] Check name
      (bind _acceptable (CallFunction|CheckNameIsAcceptable (LocalVariables|GetLocalCharacterName)))
      (if _acceptable
        ;[1 1 1] Check for available character slots
        (bind (_success _stringarray) (CallFunction|GetPlayerFile (Utilities|String|ToString(Text) (Variables|Names|GetUsername))))
        (if _success
          (bind _output_get (LocalVariables|SetPlayerFile _stringarray))
          (bind _slotavailable (CallFunction|FindAvailableCharacterSlot _output_get))
          (LocalVariables|SetLocalSlotAvailable _slotavailable)
          ;[1 1 1] Create character data
          (bind (_created _startingitems) (CallFunction|CreateStartInventory))
          (if _created
            (bind _playerstruct (CallFunction|MakePlayerStruct _startingitems (LocalVariables|GetLocalCharacterName)))
            (bind _output_get_2 (LocalVariables|SetLocalPlayerStruct _playerstruct))
            (bind (_characterdata _playerinventorystruct) (CallFunction|BuildCharacterArrayfromStruct _output_get_2))
            (LocalVariables|SetLocalCharacterStringArray _characterdata)
            (bind _inventorystring (CallFunction|BuildInventoryString _playerinventorystruct))
            (bind _success_2 (CallFunction|MakeInventoryFilefromStringArray _inventorystring (LocalVariables|GetLocalCharacterName)))
            (if _success_2
              ;[1 1 1] Save Character File
              (bind _success_3 (CallFunction|SaveCharacterFile (LocalVariables|GetLocalCharacterStringArray) (LocalVariables|GetLocalCharacterName)))
              (if _success_3
                ;[1 1 1] Make Player Database struct from csv file
                (bind _newstruct (CallFunction|StructfromDatatable)) ; Make struct from player csv file.
                (bind _newplayerdatabase (CallFunction|DatatablefromStruct _newstruct (LocalVariables|GetLocalCharacterName) (LocalVariables|GetLocalSlotAvailable))) ; Remake datatable with new info
                (bind _output_get_3 (LocalVariables|SetLocalNewPlayerDatabase _newplayerdatabase))
                ;[1 1 1] Save Character to player slot
                (bind _success_4 (CallFunction|SaveCharactertoPlayerSlot _output_get_3))
                (if _success_4
                  ;[1 1 1] Populate new character
                  (CallFunction|PopulateNewCharacter (LocalVariables|GetLocalIsMale) (Utilities|Text|ToText(String) (LocalVariables|GetLocalCharacterName)))
                  (return true)
                  (else
                    (Development|PrintString "Unable to save character to player datatable" true true "(R=0.000000,G=0.660000,B=1.000000,A=1.000000)" 1e+01)
                    (return false)))
                (else
                  (Development|PrintString "Failed to make character file!")
                  (return false)))
              (else
                (Development|PrintString "Unable to create inventory file!" true true "(R=0.000000,G=0.660000,B=1.000000,A=1.000000)" 8.0)
                (return false)))
            (else
              (Development|PrintString "CreateStartInventory in GM_CharacterSelect failed.")
              (return false)))
          (else
            (Development|PrintString "Can't find user file in GM_CharacterSelect > Create Character")
            (return false)))
        (else
          (return false))))))

(fn CheckLettersinName
  (params (NameToCheck :type String))
  (bind _output_get (LocalVariables|SetLocalStringArray (Utilities|String|GetCharacterArrayfromString (Class|KismetStringLibrary|ToUpper NameToCheck))))
  (for _array_element _output_get
    (LocalVariables|SetCharacterBeingChecked _array_element)
    (LocalVariables|SetCharacterBad (not (Utilities|Array|ContainsItem (LocalVariables|GetLocalArrayToCheckAgainst) (LocalVariables|GetCharacterBeingChecked)))))
  (return (LocalVariables|GetCharacterBad)))

(fn CreateStartInventory
  (for _array_element (Variables|Inventory|GetStarterItemNames)
    (bind _returnvalue (Utilities|GetDataTableRow "/Game/Startup/CSV/CSV_ItemDatabase.CSV_ItemDatabase" _array_element)
      (:then
        (bind _output_get (LocalVariables|SetLocalItemInLoop _returnvalue))
        (Utilities|Array|Add (LocalVariables|GetStartingItemArray) _output_get))))
  (return true (LocalVariables|GetStartingItemArray)))

(fn GearStructtoString
  (params (GearStruct :type S%20Item%20Master%20Structure))
  (Utilities|Array|Clear (Variables|Inventory|GetNewGear))
  (return (CallFunction|StringArraytoString (Variables|Inventory|GetNewGear))))

(fn BuildInventoryString
  (params (InventoryStructArray :type Array%20of%20S%20Item%20Details%20Structures))
  (Utilities|Array|Clear (LocalVariables|GetLocalInventoryStringArray))
  (for _array_element InventoryStructArray
    (Utilities|Array|Add (LocalVariables|GetLocalInventoryStringArray) (Utilities|String|Append "," (Utilities|String|JoinStringArray (Utilities|Array|MakeArray (Utilities|String|ToString(Integer) (.ItemID (Utilities|Struct|BreakS_ItemDetails _array_element))) (.ItemName (Utilities|Struct|BreakS_ItemDetails _array_element)) (.ShortDesc (Utilities|Struct|BreakS_ItemDetails _array_element)) (.LongDesc (Utilities|Struct|BreakS_ItemDetails _array_element)) (Utilities|String|ToString(Boolean) (.Equipped (Utilities|Struct|BreakS_ItemDetails _array_element))) (Utilities|String|ToString(Boolean) (.CanBeEquipped (Utilities|Struct|BreakS_ItemDetails _array_element))) (.EquipSlot (Utilities|Struct|BreakS_ItemDetails _array_element)) (Utilities|String|ToString(Boolean) (.IsWeapon (Utilities|Struct|BreakS_ItemDetails _array_element))) (.WeaponType (Utilities|Struct|BreakS_ItemDetails _array_element)) (Utilities|String|ToString(Boolean) (.IsArmor (Utilities|Struct|BreakS_ItemDetails _array_element))) (.ArmorType (Utilities|Struct|BreakS_ItemDetails _array_element)) (CallFunction|StringArraytoString (.DamageType (Utilities|Struct|BreakS_ItemDetails _array_element))) (CallFunction|StringArraytoString (.DefenseType (Utilities|Struct|BreakS_ItemDetails _array_element))) (CallFunction|StringArraytoString (.DamageBaseRange (Utilities|Struct|BreakS_ItemDetails _array_element))) (CallFunction|StringArraytoString (.ArmorBaseRange (Utilities|Struct|BreakS_ItemDetails _array_element))) (Utilities|String|ToString(Float) (.Weight (Utilities|Struct|BreakS_ItemDetails _array_element))) (Utilities|String|ToString(Float) (.Cost (Utilities|Struct|BreakS_ItemDetails _array_element))) (Utilities|String|ToString(Float) (.ItemHealth (Utilities|Struct|BreakS_ItemDetails _array_element))) (Utilities|String|ToString(Float) (.ItemMaxHealth (Utilities|Struct|BreakS_ItemDetails _array_element)))) ","))))
  (return (LocalVariables|GetLocalInventoryStringArray)))

(fn StringArraytoString
  (params (StringArray :type Array%20of%20Strings))
  (return (Utilities|String|JoinStringArray StringArray ", ")))

(fn CreateLoginWidget
  (params (NewPlayer :type Player%20Controller%20Object%20Reference))
  ;[1 1 1] Create widget for login
  (bind _output_get (Variables|References|SetNewPlayer NewPlayer))
  (bind _returnvalue (UserInterface|CreateWidget "/Game/Startup/Widgets/W_LoginScreen.W_LoginScreen_C" _output_get))
  (bind _output_get_2 (Variables|References|SetNewPlayerLoginWidget _returnvalue))
  (UserInterface|Viewport|AddtoViewport _output_get_2 0)
  (Input|SetInputModeGameandUI (Variables|References|GetNewPlayer) (Variables|References|GetNewPlayerLoginWidget) "DoNotLock" false)
  (Variables|/Script/Engine.PlayerController|SetbShowMouseCursor (Variables|References|GetNewPlayer) true))

(fn LoadCharacterSelection
  (params (Player :type Player%20Controller%20Object%20Reference) (Username :type Text))
  ;[0.7747 1 0.7885] Check if username in datatable
  (Variables|References|SetNewPlayer Player)
  (bind _output_get (Variables|Names|SetUsername Username))
  (bind _path (CallFunction|FindSaveFile "CSV" (Utilities|String|ToString(Text) _output_get)))
  (bind (_stringarray _returnvalue) (Class|TextFileManager|LoadArrayText (.path _path)))
  (if _returnvalue
    (bind _output_get_2 (LocalVariables|SetLocalCharacterFileArray _stringarray))
    (bind _parsedarray (CallFunction|ParseCleanArray 1 _output_get_2))
    (Utilities|Array|RemoveIndex _parsedarray)
    (Utilities|Array|RemoveIndex _parsedarray 1)
    (bind _output_get_3 (LocalVariables|SetLocalSlotsArray _parsedarray))
    (return _output_get_3)
    (else
      (Development|PrintString "Can't find user file in GM_CharacterSelect > LoadCharacterSelection" true true "(R=0.000000,G=0.660000,B=1.000000,A=1.000000)" 6.0))))

(fn StructfromDatatable
  (bind (_stringarray _returnvalue) (Class|TextFileManager|LoadArrayText (Utilities|String|Append (Utilities|Struct|BreakDirectoryPath (Variables|FilePaths|GetCSVSaveDirectory)) "/" (Utilities|String|ToString(Text) (Variables|Names|GetUsername)) ".csv")))
  (bind _parsedarray (CallFunction|ParseCleanArray 1 _stringarray))
  (if _returnvalue
    (bind _output_get (LocalVariables|SetLocalNewPlayerDatabase (Utilities|Struct|MakeS_Player_Datatable (Math|Conversions|ToInteger(Byte) (Utilities|Array|Get(acopy) _parsedarray)) (Utilities|Array|Get(acopy) _parsedarray 1) (Utilities|Array|Get(acopy) _parsedarray 2) (Utilities|Array|Get(acopy) _parsedarray 3) (Utilities|Array|Get(acopy) _parsedarray 4) (Utilities|Array|Get(acopy) _parsedarray 5))))
    (return _output_get)
    (else
      (Development|PrintString "Unable to access player data table in GM_CharacterSelect > StructFromDatatable"))))

(fn DatatablefromStruct
  (params (Struct :type S%20Player%20Datatable%20Structure) (NewCharacterName :type String) (SlotAvailable :type Integer))
  (LocalVariables|SetLocalNewPlayerDatabase Struct)
  (LocalVariables|SetLocal_NewCharacterName NewCharacterName)
  (if (== SlotAvailable 3)
    (Utilities|Struct|SetmembersinS_Player_Datatable (LocalVariables|GetLocalNewPlayerDatabase) (LocalVariables|GetLocal_NewCharacterName))
    (return (LocalVariables|GetLocalNewPlayerDatabase))
    (elif (== SlotAvailable 4)
      (Utilities|Struct|SetmembersinS_Player_Datatable (LocalVariables|GetLocalNewPlayerDatabase) (LocalVariables|GetLocal_NewCharacterName))
      (return (LocalVariables|GetLocalNewPlayerDatabase))
      (elif (== SlotAvailable 5)
        (Utilities|Struct|SetmembersinS_Player_Datatable (LocalVariables|GetLocalNewPlayerDatabase) (LocalVariables|GetLocal_NewCharacterName))
        (return (LocalVariables|GetLocalNewPlayerDatabase))
        (elif (== SlotAvailable 6)
          (Utilities|Struct|SetmembersinS_Player_Datatable (LocalVariables|GetLocalNewPlayerDatabase) (LocalVariables|GetLocal_NewCharacterName))
          (return (LocalVariables|GetLocalNewPlayerDatabase))
          (else
            (Development|PrintString "No index found in GM_CharacterSelect > DatatableFromStruct")))))))

(fn BuildCharacterArrayfromStruct
  (params (PlayerStruct :type S%20Player%20Saves%20Structure))
  (LocalVariables|SetLocalPlayerStruct PlayerStruct)
  (Utilities|Array|Add (LocalVariables|GetLocalCharacterStringArray) (LocalVariables|GetLocalHeaderString))
  (bind _result (Utilities|Set|ToArray (Utilities|Set|MakeSet (Utilities|String|ToString(Text) (.playername (LocalVariables|GetLocalPlayerStruct))) (Utilities|String|ToString(Float) (.health (LocalVariables|GetLocalPlayerStruct))) (Utilities|String|ToString(Float) (.maxhealth (LocalVariables|GetLocalPlayerStruct))) (Utilities|String|ToString(Float) (.hunger (LocalVariables|GetLocalPlayerStruct))) (Utilities|String|ToString(Float) (.maxhunger (LocalVariables|GetLocalPlayerStruct))) (Utilities|String|ToString(Float) (.thirst (LocalVariables|GetLocalPlayerStruct))) (Utilities|String|ToString(Float) (.maxthirst (LocalVariables|GetLocalPlayerStruct))) (Utilities|String|ToString(Float) (.stamina (LocalVariables|GetLocalPlayerStruct))) (Utilities|String|ToString(Float) (.maxstamina (LocalVariables|GetLocalPlayerStruct))) (Utilities|String|ToString(Integer) (.level (LocalVariables|GetLocalPlayerStruct))) (Utilities|String|ToString(Integer) (.exp (LocalVariables|GetLocalPlayerStruct))) (Utilities|String|ToString(Integer) (.statpoints (LocalVariables|GetLocalPlayerStruct))) (CallFunction|GearStructtoString (.equippedhead (LocalVariables|GetLocalPlayerStruct))) (CallFunction|GearStructtoString (.equippedchest (LocalVariables|GetLocalPlayerStruct))) (CallFunction|GearStructtoString (.equippedarms (LocalVariables|GetLocalPlayerStruct))) (CallFunction|GearStructtoString (.equippedbottom (LocalVariables|GetLocalPlayerStruct))) (CallFunction|GearStructtoString (.equippedfeet (LocalVariables|GetLocalPlayerStruct))) (CallFunction|GearStructtoString (.equippedrighthand (LocalVariables|GetLocalPlayerStruct))) (CallFunction|GearStructtoString (.equippedlefthand (LocalVariables|GetLocalPlayerStruct))) (CallFunction|GearStructtoString (.equippedbag (LocalVariables|GetLocalPlayerStruct))) (Utilities|String|ToString(Float) (.currentspeed (LocalVariables|GetLocalPlayerStruct))) (Utilities|String|ToString(Float) (.maxspeed (LocalVariables|GetLocalPlayerStruct))) (CallFunction|StringArraytoString (.ownedmounts (LocalVariables|GetLocalPlayerStruct))) (CallFunction|StringArraytoString (.ownedpets (LocalVariables|GetLocalPlayerStruct))) (.playerclass (LocalVariables|GetLocalPlayerStruct)) (Utilities|String|ToString(Integer) (.strength (LocalVariables|GetLocalPlayerStruct))) (Utilities|String|ToString(Integer) (.agility (LocalVariables|GetLocalPlayerStruct))) (Utilities|String|ToString(Integer) (.constitution (LocalVariables|GetLocalPlayerStruct))))))
  (Utilities|Array|Add (LocalVariables|GetLocalCharacterStringArray) (Utilities|String|Append "," (Utilities|String|JoinStringArray _result ",")))
  (return (LocalVariables|GetLocalCharacterStringArray) (.inventory (LocalVariables|GetLocalPlayerStruct))))

(fn MakeInventoryFilefromStringArray
  (params (Inventory%20String :type Array%20of%20Strings) (CharacterName :type String))
  (Variables|Inventory|SetInventory%20String Inventory%20String)
  (bind _returnvalue (Class|TextFileManager|SaveArrayText (Utilities|String|Append (Utilities|Struct|BreakDirectoryPath (Variables|FilePaths|GetServerSaveDirectory)) "/Inventory/") (Utilities|String|Append CharacterName "_Inventory.csv") (Variables|Inventory|GetInventory%20String) true))
  (return _returnvalue))

(fn CheckNameIsAcceptable
  (params (Name :type String))
  (if (Math|Integer|InRange(Integer) (Utilities|String|Len Name) 5 10)
    (if (CallFunction|CheckLettersinName Name)
      (Development|PrintString "Name must only contain letters.")
      (return false)
      (else
        (return true)))
    (else
      (Development|PrintString "Name must be between 5 and 10 characters."))))

(fn SearchCharacterNameinPlayerDB
  (params (CharacterName :type String))
  (bind _serversavedirectory (Variables|FilePaths|GetServerSaveDirectory))
  (bind _path (Utilities|Struct|BreakDirectoryPath _serversavedirectory))
  (bind _returnvalue (Utilities|String|Append _path "/Characters/" CharacterName ".csv"))
  (bind _returnvalue_2 (Class|BlueprintPathsLibrary|FileExists _returnvalue))
  ;[1 1 1] Comment
  (if _returnvalue_2
    _
    (else
      _))
  (return _returnvalue_2))

(fn SpawnMainCharacterinSelectionScreen
  (params (StartupCharacterViewer :type BP%20Startup%20Character%20Viewer%20Object%20Reference))
  ;[1 1 1] Get StartupCharacterViewer location and spawn MainCharacter based on that
  (bind _returnvalue (Game|SpawnActorfromClass "/Game/Startup/Characters/BP_MainCharacter.BP_MainCharacter_C" (Math|Transform|MakeTransform (+ (Transformation|GetWorldLocation (Variables|/Script/Engine.Character|GetMesh StartupCharacterViewer)) "700.000000,50.000000,300.000000") "0,160.000000, 0") "AlwaysSpawn" 0 0))
  (bind _output_get (Variables|References|SetMain%20Character%20Ref _returnvalue))
  (return (Utilities|IsValid _output_get)))

(fn CreateCharacterSelectionScreenWidget
  (params (CharacterSlotArray :type Array%20of%20Strings))
  ;[1 1 1] Create character selection widget
  (LocalVariables|SetLocalSlotsArray CharacterSlotArray)
  (bind _returnvalue (UserInterface|CreateWidget "/Game/Startup/Widgets/W_CharacterSelection.W_CharacterSelection_C" (Variables|References|GetNewPlayer) (Variables|References|GetMain%20Character%20Ref)))
  (bind _output_get (Variables|References|SetSelectionWidgetRef _returnvalue))
  (UserInterface|Viewport|AddtoViewport _output_get 0)
  (Variables|/Script/Engine.PlayerController|SetbShowMouseCursor (Variables|References|GetNewPlayer) true)
  ;[1 1 1] Create a button for each available character
  (for _array_element (LocalVariables|GetLocalSlotsArray)
    (if (not (<= (Utilities|String|Len _array_element) 0))
      (bind _returnvalue_2 (UserInterface|CreateWidget "/Game/Startup/Widgets/W_CharacterSelectionButtons.W_CharacterSelectionButtons_C" (Variables|References|GetNewPlayer)))
      (Rendering|Components|TextRender|SetText (Variables|/Game/Startup/Widgets/W_CharacterSelectionButtons.W_CharacterSelectionButtons_C|GetCharacterChoiceText _returnvalue_2) (Utilities|Text|ToText(String) _array_element))
      (Default|AddCharacterButton (Variables|References|GetSelectionWidgetRef) _returnvalue_2)))
  (return))

(fn GetNewUser
  (params (Username :type Text) (Password :type Text) (LoginWidget :type W%20Login%20Screen%20Object%20Reference))
  ;[1 1 1] Check if username already exists
  (Variables|Names|SetUsername Username)
  (Variables|References|SetNewPlayerLoginWidget LoginWidget)
  (bind _fileexists (CallFunction|FindSaveFile "CSV" (Utilities|String|ToString(Text) (Variables|Names|GetUsername))))
  (if _fileexists
    (Development|PrintString "Username already exists.")
    (else
      ;[1 1 1] Setup user data for saving to file
      (LocalVariables|SetLocalUserData (Utilities|Array|MakeArray "Index,Username,Slot1,Slot2,Slot3,Slot4" (Utilities|String|Append (Utilities|String|ToString(Integer) (Class|GameplayStatics|GetPlayerControllerID (Variables|References|GetNewPlayer))) "," (Utilities|String|ToString(Text) (Variables|Names|GetUsername)))))
      ;[1 1 1] Save data to new user file
      (bind _returnvalue (Class|TextFileManager|SaveArrayText (.path (Variables|FilePaths|GetCSVSaveDirectory)) (Utilities|String|Append (Utilities|String|ToString(Text) (Variables|Names|GetUsername)) ".csv") (LocalVariables|GetLocalUserData) true))
      (return _returnvalue))))

(fn CreateStartupCharacterViewer
  (params (Player :type Player%20Controller%20Object%20Reference))
  ;[1 1 1] Spawn StartupCharacterViewer
  (bind _returnvalue (Game|SpawnActorfromClass "/Game/Startup/Characters/BP_StartupCharacterViewer.BP_StartupCharacterViewer_C" (Math|Transform|MakeTransform "0, 0, 0") "AlwaysSpawn" Player 0))
  (bind _output_get (Variables|References|SetBP_StartupCharacterViewer _returnvalue))
  (return (Utilities|IsValid _output_get)))

(fn PopulateNewCharacter
  (params (IsMale :type Boolean) (CharacterName :type Text))
  (bind _main_character_ref (Variables|References|GetMain%20Character%20Ref))
  (Input|SetInputModeGameOnly (Variables|References|GetNewPlayer))
  (Variables|/Game/Startup/Characters/BP_MainCharacter.BP_MainCharacter_C|SetIsMale _main_character_ref IsMale)
  (Variables|/Game/Startup/Characters/BP_MainCharacter.BP_MainCharacter_C|SetPlayerName _main_character_ref CharacterName)
  (Pawn|Possess (Variables|References|GetNewPlayer) _main_character_ref)
  (return))

(fn CheckCharacterExists
  (params (CharacterName :type String))
  (return (Class|BlueprintPathsLibrary|FileExists (Utilities|String|Append (Utilities|Struct|BreakDirectoryPath (Variables|FilePaths|GetServerSaveDirectory)) "/Characters/" (Utilities|String|Append CharacterName ".csv")))))

(fn GetPlayerFile
  (params (Username :type String))
  (bind (_stringarray _returnvalue) (Class|TextFileManager|LoadArrayText (Utilities|String|Append (Utilities|Struct|BreakDirectoryPath (Variables|FilePaths|GetCSVSaveDirectory)) "/" (Utilities|String|Append Username ".csv"))))
  (return _returnvalue _stringarray))

(fn FindAvailableCharacterSlot
  (params (FileArray :type Array%20of%20Strings))
  (bind _parsedarray (CallFunction|ParseCleanArray 1 FileArray))
  (if (<= (Utilities|String|Len (Utilities|Array|Get(acopy) _parsedarray 2)) 0)
    (LocalVariables|SetLocalSlotAvailable 3) ; Slot avilable is index of array item + 1, since first array item is technically a 0.
    (return (LocalVariables|GetLocalSlotAvailable))
    (elif (<= (Utilities|String|Len (Utilities|Array|Get(acopy) _parsedarray 3)) 0)
      (LocalVariables|SetLocalSlotAvailable 4)
      (return (LocalVariables|GetLocalSlotAvailable))
      (elif (<= (Utilities|String|Len (Utilities|Array|Get(acopy) _parsedarray 4)) 0)
        (LocalVariables|SetLocalSlotAvailable 5)
        (return (LocalVariables|GetLocalSlotAvailable))
        (elif (<= (Utilities|String|Len (Utilities|Array|Get(acopy) _parsedarray 5)) 0)
          (LocalVariables|SetLocalSlotAvailable 6)
          (return (LocalVariables|GetLocalSlotAvailable)))))))

(fn MakePlayerStruct
  (params (StartingItems :type Array%20of%20S%20Item%20Details%20Structures) (CharacterName :type String))
  (bind _output_get (Variables|Inventory|SetStarting%20Items StartingItems))
  (bind _structout (Utilities|Struct|SetmembersinS_PlayerSaves (Utilities|Struct|MakeS_PlayerSaves (Utilities|Text|ToText(String) CharacterName) 6e+01 6e+01 1e+02 1e+02 1e+02 1e+02 6e+01 6e+01 1 0 5 _output_get "(Item_6_F556053D47D34E54984CEFA1D6C68729=(ItemID_2_19E77F0A4482006853C426BFC8A35FF9=0,ItemName_8_DBD8193A4220BBD3C379BA8C95A6C070=\"Stone Knife\",ShortDesc_9_1AD59278445FA9B955FF65BD6818A0FC=\"A crude knife.\",LongDesc_11_24424878454602FA6B485689018FEF34=\"A simple, crude knife made of stone and a stick.\",Equipped_14_41B8598C449BFAAE0B59C980DC9E5EA1=False,CanBeEquipped_19_F24D8BFE410763AC7A5B038AD49601FE=True,EquipSlot_20_DD358362424D213B5ED1298889A88050=\"RightHand\",IsWeapon_23_33C65F404B6FBEFE5BC94387BDF985A8=False,WeaponType_26_3BBACC5145C79CD4DB414FB5515C9542=\"Blade\",IsArmor_29_518DB92F4BB5DFDC74EA12932E91CA17=False,ArmorType_32_DCA3D0E541E3A6F386502C88C78FA817=\"\",DamageType_36_417C9C854CEE0C73E57575AC28D7BDC3=(\"Pierce\",\"Slash\"),DefenseType_38_256A68A241079F8CF4EB048D4B7B8AB6=(\"Physical\"),DamageBaseRange_65_F6229E894D40F8CAA470F984FFAF9049=(\"1\",\"2\"),ArmorBaseRange_66_221C47F24F6BBC2A6D342F911ED54DA9=(\"0\",\"0\"),Weight_54_011C13344C6FA211655277B30EFF0771=1.000000,Cost_56_AE8A67574D4EE12168A93F8904AF5ED1=1.500000,ItemHealth_58_E0B1D3AD472CF7EC29210EA60AD75DDF=50.000000,ItemMaxHealth_60_DA9DB1154F30DAEB15C316BCC1823E9C=50.000000))" "(Item_6_F556053D47D34E54984CEFA1D6C68729=(ItemID_2_19E77F0A4482006853C426BFC8A35FF9=0,ItemName_8_DBD8193A4220BBD3C379BA8C95A6C070=\"Stone Knife\",ShortDesc_9_1AD59278445FA9B955FF65BD6818A0FC=\"A crude knife.\",LongDesc_11_24424878454602FA6B485689018FEF34=\"A simple, crude knife made of stone and a stick.\",Equipped_14_41B8598C449BFAAE0B59C980DC9E5EA1=False,CanBeEquipped_19_F24D8BFE410763AC7A5B038AD49601FE=True,EquipSlot_20_DD358362424D213B5ED1298889A88050=\"RightHand\",IsWeapon_23_33C65F404B6FBEFE5BC94387BDF985A8=False,WeaponType_26_3BBACC5145C79CD4DB414FB5515C9542=\"Blade\",IsArmor_29_518DB92F4BB5DFDC74EA12932E91CA17=False,ArmorType_32_DCA3D0E541E3A6F386502C88C78FA817=\"\",DamageType_36_417C9C854CEE0C73E57575AC28D7BDC3=(\"Pierce\",\"Slash\"),DefenseType_38_256A68A241079F8CF4EB048D4B7B8AB6=(\"Physical\"),DamageBaseRange_65_F6229E894D40F8CAA470F984FFAF9049=(\"1\",\"2\"),ArmorBaseRange_66_221C47F24F6BBC2A6D342F911ED54DA9=(\"0\",\"0\"),Weight_54_011C13344C6FA211655277B30EFF0771=1.000000,Cost_56_AE8A67574D4EE12168A93F8904AF5ED1=1.500000,ItemHealth_58_E0B1D3AD472CF7EC29210EA60AD75DDF=50.000000,ItemMaxHealth_60_DA9DB1154F30DAEB15C316BCC1823E9C=50.000000))" "(Item_6_F556053D47D34E54984CEFA1D6C68729=(ItemID_2_19E77F0A4482006853C426BFC8A35FF9=0,ItemName_8_DBD8193A4220BBD3C379BA8C95A6C070=\"Stone Knife\",ShortDesc_9_1AD59278445FA9B955FF65BD6818A0FC=\"A crude knife.\",LongDesc_11_24424878454602FA6B485689018FEF34=\"A simple, crude knife made of stone and a stick.\",Equipped_14_41B8598C449BFAAE0B59C980DC9E5EA1=False,CanBeEquipped_19_F24D8BFE410763AC7A5B038AD49601FE=True,EquipSlot_20_DD358362424D213B5ED1298889A88050=\"RightHand\",IsWeapon_23_33C65F404B6FBEFE5BC94387BDF985A8=False,WeaponType_26_3BBACC5145C79CD4DB414FB5515C9542=\"Blade\",IsArmor_29_518DB92F4BB5DFDC74EA12932E91CA17=False,ArmorType_32_DCA3D0E541E3A6F386502C88C78FA817=\"\",DamageType_36_417C9C854CEE0C73E57575AC28D7BDC3=(\"Pierce\",\"Slash\"),DefenseType_38_256A68A241079F8CF4EB048D4B7B8AB6=(\"Physical\"),DamageBaseRange_65_F6229E894D40F8CAA470F984FFAF9049=(\"1\",\"2\"),ArmorBaseRange_66_221C47F24F6BBC2A6D342F911ED54DA9=(\"0\",\"0\"),Weight_54_011C13344C6FA211655277B30EFF0771=1.000000,Cost_56_AE8A67574D4EE12168A93F8904AF5ED1=1.500000,ItemHealth_58_E0B1D3AD472CF7EC29210EA60AD75DDF=50.000000,ItemMaxHealth_60_DA9DB1154F30DAEB15C316BCC1823E9C=50.000000))" "(Item_6_F556053D47D34E54984CEFA1D6C68729=(ItemID_2_19E77F0A4482006853C426BFC8A35FF9=0,ItemName_8_DBD8193A4220BBD3C379BA8C95A6C070=\"Stone Knife\",ShortDesc_9_1AD59278445FA9B955FF65BD6818A0FC=\"A crude knife.\",LongDesc_11_24424878454602FA6B485689018FEF34=\"A simple, crude knife made of stone and a stick.\",Equipped_14_41B8598C449BFAAE0B59C980DC9E5EA1=False,CanBeEquipped_19_F24D8BFE410763AC7A5B038AD49601FE=True,EquipSlot_20_DD358362424D213B5ED1298889A88050=\"RightHand\",IsWeapon_23_33C65F404B6FBEFE5BC94387BDF985A8=False,WeaponType_26_3BBACC5145C79CD4DB414FB5515C9542=\"Blade\",IsArmor_29_518DB92F4BB5DFDC74EA12932E91CA17=False,ArmorType_32_DCA3D0E541E3A6F386502C88C78FA817=\"\",DamageType_36_417C9C854CEE0C73E57575AC28D7BDC3=(\"Pierce\",\"Slash\"),DefenseType_38_256A68A241079F8CF4EB048D4B7B8AB6=(\"Physical\"),DamageBaseRange_65_F6229E894D40F8CAA470F984FFAF9049=(\"1\",\"2\"),ArmorBaseRange_66_221C47F24F6BBC2A6D342F911ED54DA9=(\"0\",\"0\"),Weight_54_011C13344C6FA211655277B30EFF0771=1.000000,Cost_56_AE8A67574D4EE12168A93F8904AF5ED1=1.500000,ItemHealth_58_E0B1D3AD472CF7EC29210EA60AD75DDF=50.000000,ItemMaxHealth_60_DA9DB1154F30DAEB15C316BCC1823E9C=50.000000))" "(Item_6_F556053D47D34E54984CEFA1D6C68729=(ItemID_2_19E77F0A4482006853C426BFC8A35FF9=0,ItemName_8_DBD8193A4220BBD3C379BA8C95A6C070=\"Stone Knife\",ShortDesc_9_1AD59278445FA9B955FF65BD6818A0FC=\"A crude knife.\",LongDesc_11_24424878454602FA6B485689018FEF34=\"A simple, crude knife made of stone and a stick.\",Equipped_14_41B8598C449BFAAE0B59C980DC9E5EA1=False,CanBeEquipped_19_F24D8BFE410763AC7A5B038AD49601FE=True,EquipSlot_20_DD358362424D213B5ED1298889A88050=\"RightHand\",IsWeapon_23_33C65F404B6FBEFE5BC94387BDF985A8=False,WeaponType_26_3BBACC5145C79CD4DB414FB5515C9542=\"Blade\",IsArmor_29_518DB92F4BB5DFDC74EA12932E91CA17=False,ArmorType_32_DCA3D0E541E3A6F386502C88C78FA817=\"\",DamageType_36_417C9C854CEE0C73E57575AC28D7BDC3=(\"Pierce\",\"Slash\"),DefenseType_38_256A68A241079F8CF4EB048D4B7B8AB6=(\"Physical\"),DamageBaseRange_65_F6229E894D40F8CAA470F984FFAF9049=(\"1\",\"2\"),ArmorBaseRange_66_221C47F24F6BBC2A6D342F911ED54DA9=(\"0\",\"0\"),Weight_54_011C13344C6FA211655277B30EFF0771=1.000000,Cost_56_AE8A67574D4EE12168A93F8904AF5ED1=1.500000,ItemHealth_58_E0B1D3AD472CF7EC29210EA60AD75DDF=50.000000,ItemMaxHealth_60_DA9DB1154F30DAEB15C316BCC1823E9C=50.000000))" "(Item_6_F556053D47D34E54984CEFA1D6C68729=(ItemID_2_19E77F0A4482006853C426BFC8A35FF9=0,ItemName_8_DBD8193A4220BBD3C379BA8C95A6C070=\"Stone Knife\",ShortDesc_9_1AD59278445FA9B955FF65BD6818A0FC=\"A crude knife.\",LongDesc_11_24424878454602FA6B485689018FEF34=\"A simple, crude knife made of stone and a stick.\",Equipped_14_41B8598C449BFAAE0B59C980DC9E5EA1=False,CanBeEquipped_19_F24D8BFE410763AC7A5B038AD49601FE=True,EquipSlot_20_DD358362424D213B5ED1298889A88050=\"RightHand\",IsWeapon_23_33C65F404B6FBEFE5BC94387BDF985A8=False,WeaponType_26_3BBACC5145C79CD4DB414FB5515C9542=\"Blade\",IsArmor_29_518DB92F4BB5DFDC74EA12932E91CA17=False,ArmorType_32_DCA3D0E541E3A6F386502C88C78FA817=\"\",DamageType_36_417C9C854CEE0C73E57575AC28D7BDC3=(\"Pierce\",\"Slash\"),DefenseType_38_256A68A241079F8CF4EB048D4B7B8AB6=(\"Physical\"),DamageBaseRange_65_F6229E894D40F8CAA470F984FFAF9049=(\"1\",\"2\"),ArmorBaseRange_66_221C47F24F6BBC2A6D342F911ED54DA9=(\"0\",\"0\"),Weight_54_011C13344C6FA211655277B30EFF0771=1.000000,Cost_56_AE8A67574D4EE12168A93F8904AF5ED1=1.500000,ItemHealth_58_E0B1D3AD472CF7EC29210EA60AD75DDF=50.000000,ItemMaxHealth_60_DA9DB1154F30DAEB15C316BCC1823E9C=50.000000))" "(Item_6_F556053D47D34E54984CEFA1D6C68729=(ItemID_2_19E77F0A4482006853C426BFC8A35FF9=0,ItemName_8_DBD8193A4220BBD3C379BA8C95A6C070=\"Stone Knife\",ShortDesc_9_1AD59278445FA9B955FF65BD6818A0FC=\"A crude knife.\",LongDesc_11_24424878454602FA6B485689018FEF34=\"A simple, crude knife made of stone and a stick.\",Equipped_14_41B8598C449BFAAE0B59C980DC9E5EA1=False,CanBeEquipped_19_F24D8BFE410763AC7A5B038AD49601FE=True,EquipSlot_20_DD358362424D213B5ED1298889A88050=\"RightHand\",IsWeapon_23_33C65F404B6FBEFE5BC94387BDF985A8=False,WeaponType_26_3BBACC5145C79CD4DB414FB5515C9542=\"Blade\",IsArmor_29_518DB92F4BB5DFDC74EA12932E91CA17=False,ArmorType_32_DCA3D0E541E3A6F386502C88C78FA817=\"\",DamageType_36_417C9C854CEE0C73E57575AC28D7BDC3=(\"Pierce\",\"Slash\"),DefenseType_38_256A68A241079F8CF4EB048D4B7B8AB6=(\"Physical\"),DamageBaseRange_65_F6229E894D40F8CAA470F984FFAF9049=(\"1\",\"2\"),ArmorBaseRange_66_221C47F24F6BBC2A6D342F911ED54DA9=(\"0\",\"0\"),Weight_54_011C13344C6FA211655277B30EFF0771=1.000000,Cost_56_AE8A67574D4EE12168A93F8904AF5ED1=1.500000,ItemHealth_58_E0B1D3AD472CF7EC29210EA60AD75DDF=50.000000,ItemMaxHealth_60_DA9DB1154F30DAEB15C316BCC1823E9C=50.000000))" "(Item_6_F556053D47D34E54984CEFA1D6C68729=(ItemID_2_19E77F0A4482006853C426BFC8A35FF9=0,ItemName_8_DBD8193A4220BBD3C379BA8C95A6C070=\"Stone Knife\",ShortDesc_9_1AD59278445FA9B955FF65BD6818A0FC=\"A crude knife.\",LongDesc_11_24424878454602FA6B485689018FEF34=\"A simple, crude knife made of stone and a stick.\",Equipped_14_41B8598C449BFAAE0B59C980DC9E5EA1=False,CanBeEquipped_19_F24D8BFE410763AC7A5B038AD49601FE=True,EquipSlot_20_DD358362424D213B5ED1298889A88050=\"RightHand\",IsWeapon_23_33C65F404B6FBEFE5BC94387BDF985A8=False,WeaponType_26_3BBACC5145C79CD4DB414FB5515C9542=\"Blade\",IsArmor_29_518DB92F4BB5DFDC74EA12932E91CA17=False,ArmorType_32_DCA3D0E541E3A6F386502C88C78FA817=\"\",DamageType_36_417C9C854CEE0C73E57575AC28D7BDC3=(\"Pierce\",\"Slash\"),DefenseType_38_256A68A241079F8CF4EB048D4B7B8AB6=(\"Physical\"),DamageBaseRange_65_F6229E894D40F8CAA470F984FFAF9049=(\"1\",\"2\"),ArmorBaseRange_66_221C47F24F6BBC2A6D342F911ED54DA9=(\"0\",\"0\"),Weight_54_011C13344C6FA211655277B30EFF0771=1.000000,Cost_56_AE8A67574D4EE12168A93F8904AF5ED1=1.500000,ItemHealth_58_E0B1D3AD472CF7EC29210EA60AD75DDF=50.000000,ItemMaxHealth_60_DA9DB1154F30DAEB15C316BCC1823E9C=50.000000))" 6e+02 1e+03 0 0 (Variables|Names|GetNewCharacterClass) 3 3 3)))
  (return _structout))

(fn SaveCharacterFile
  (params (CharacterData :type Array%20of%20Strings) (CharacterName :type String))
  (bind _returnvalue (Class|TextFileManager|SaveArrayText (Utilities|String|Append (Utilities|Struct|BreakDirectoryPath (Variables|FilePaths|GetServerSaveDirectory)) "/Characters/") (Utilities|String|Append CharacterName ".csv") CharacterData true))
  (return _returnvalue))

(fn SaveCharactertoPlayerSlot
  (params (PlayerStruct :type S%20Player%20Datatable%20Structure))
  (LocalVariables|SetLocalNewPlayerDatabase PlayerStruct)
  (bind _returnvalue (Class|TextFileManager|SaveArrayText (Utilities|Struct|BreakDirectoryPath (Variables|FilePaths|GetCSVSaveDirectory)) (Utilities|String|Append "/" (Utilities|String|ToString(Text) (Variables|Names|GetUsername)) ".csv") (Utilities|Array|MakeArray "Index,Username,Slot1,Slot2,Slot3,Slot4" (Utilities|String|JoinStringArray (Utilities|Array|MakeArray (Utilities|String|ToString(Integer) (.playerid (LocalVariables|GetLocalNewPlayerDatabase))) (.username (LocalVariables|GetLocalNewPlayerDatabase)) (.character1 (LocalVariables|GetLocalNewPlayerDatabase)) (.character2 (LocalVariables|GetLocalNewPlayerDatabase)) (.character3 (LocalVariables|GetLocalNewPlayerDatabase)) (.character4 (LocalVariables|GetLocalNewPlayerDatabase))) ",")) true))
  (return _returnvalue))

(fn LoadPlayerHUD
  (bind _newplayer (Variables|References|GetNewPlayer))
  ;[1 1 1] Create Health/Stamina/Etc bars
  (bind _returnvalue (UserInterface|CreateWidget "/Game/Startup/Widgets/W_CharacterOverhead.W_CharacterOverhead_C" (Variables|References|GetNewPlayer) (Variables|References|GetMain%20Character%20Ref)))
  (UserInterface|Viewport|AddtoViewport _returnvalue 0)
  ;[1 1 1] Set input mode
  (Input|SetInputModeGameOnly _newplayer)
  (Variables|/Script/Engine.PlayerController|SetbShowMouseCursor _newplayer false)
  ;[1 1 1] Remove Selection Screen Widget
  (Widget|RemovefromParent (Variables|References|GetSelectionWidgetRef)))

(fn LoadSelectedPlayer
  (params (Name :type String))
  (bind _output_get (LocalVariables|SetLocalCharacterName Name))
  (bind _nameindatabase (CallFunction|SearchCharacterNameinPlayerDB _output_get))
  (if _nameindatabase
    (Development|PrintString "Character found, however this function is currently incomplete.")
    (else
      (Development|PrintString "Can't find character save file." true true "(R=0.000000,G=0.660000,B=1.000000,A=1.000000)" 6.0))))