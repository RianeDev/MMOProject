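; MainGameState handles account login, registration and character creation, using CSV save files as the database.
; Login and registration check only usernames, never passwords, then spawn a preview character and open the slot selection widget.
; Character creation validates the name, writes character, starter inventory (from a DataTable) and user files, then calls EnterGameWorld.
; The preview's gender mesh swap runs only on the Remote branch, and StringArrayToString is an empty stub.
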(event Custom|PlayerLogin
  (params (PlayerController :type Main%20Player%20Controller%20Object%20Reference) (Username :type String) (Password :type String))
  ;[1 1 1] Attempt to login player
  (bind _success (CallFunction|AttemptLogin PlayerController Username Password))
  (if (not _success)
    (Default|GetServerMessage PlayerController "Unable to complete player login.")))

(event Custom|PlayerRegistry
  (params (PlayerController :type Main%20Player%20Controller%20Object%20Reference) (NewName :type String) (NewPassword :type String))
  ;[1 1 1] Attempt to register player
  (bind _success (CallFunction|AttemptRegistry PlayerController NewName NewPassword))
  (if (not _success)
    (Default|GetServerMessage PlayerController "Unable to complete player registry.")))

(event Custom|CreateCharacter
  (params (PlayerController :type Main%20Player%20Controller%20Object%20Reference) (UserName :type String) (CharacterName :type String) (IsMale :type Boolean))
  ;[1 1 1] Attempt to create new Character
  (bind _success (CallFunction|AttemptCreateCharacter PlayerController UserName CharacterName IsMale))
  (if _success
    (Default|GetServerMessage PlayerController "Successfully created character, loading into game...")
    (bind _success_2 (CallFunction|LoadCharacterIntoGame UserName CharacterName PlayerController))
    (if _success_2
      _)))

(event Custom|ChangeMainCharacterMesh
  (params (PlayerController :type Main%20Player%20Controller%20Object%20Reference) (MakeMale :type Boolean))
  (bind _creationcharacterref (Variables|/Game/Startup/MainPlayerController.MainPlayerController_C|GetCreationCharacterRef PlayerController))
  (bind _mesh (Variables|/Script/Engine.Character|GetMesh _creationcharacterref))
  (bind _mesh_2 (Variables|/Script/Engine.Character|GetMesh _creationcharacterref))
  ;[1 1 1] Change ManCharacter Mesh appearance
  (Networking|SwitchHasAuthority
    (:Remote
      (if (Utilities|IsValid PlayerController)
        (if MakeMale
          (if (not (Variables|/Game/Startup/Characters/BP_CreationCharacter.BP_CreationCharacter_C|GetIsMale _creationcharacterref))
            (Class|SkinnedMeshComponent|SetSkeletalMesh _mesh_2 "/Game/Mannequin/Character/Mesh/SK_Mannequin.SK_Mannequin" true)
            (Class|SkeletalMeshComponent|SetAnimClass _mesh_2 "/Game/Mannequin/Animations/ThirdPerson_AnimBP.ThirdPerson_AnimBP_C")
            (Variables|/Game/Startup/Characters/BP_CreationCharacter.BP_CreationCharacter_C|SetIsMale _creationcharacterref true))
          (elif (Variables|/Game/Startup/Characters/BP_CreationCharacter.BP_CreationCharacter_C|GetIsMale _creationcharacterref)
            (Class|SkinnedMeshComponent|SetSkeletalMesh _mesh "/Game/Mannequin/Character/Mesh/SK_Mannequin_Female.SK_Mannequin_Female" true)
            (Class|SkeletalMeshComponent|SetAnimClass _mesh "/Game/Mannequin/Animations/ThirdPerson_AnimBP.ThirdPerson_AnimBP_C")
            (Variables|/Game/Startup/Characters/BP_CreationCharacter.BP_CreationCharacter_C|SetIsMale _creationcharacterref false)))
        (else
          (Development|PrintString "CreationCharacterRef is NOT valid"))))))

(fn ConstructionScript)

(fn AttemptLogin
  (params (PlayerController :type Main%20Player%20Controller%20Object%20Reference) (Username :type String) (Password :type String))
  (LocalVariables|SetLocalPlayerController PlayerController)
  (LocalVariables|SetLocalUserName Username)
  (LocalVariables|SetLocalPassword Password)
  (bind (_path _fileexists) (CallFunction|FindSaveFile "CSV" (LocalVariables|GetLocalUserName)))
  (Development|PrintString (.path _path) true true "(R=0.000000,G=0.660000,B=1.000000,A=1.000000)" 3e+01)
  (if _fileexists
    (bind _success (CallFunction|GetCharacterSelection (LocalVariables|GetLocalPlayerController) (LocalVariables|GetLocalUserName)))
    (if _success
      (Default|GetServerMessage (LocalVariables|GetLocalPlayerController) "Character selection completed.")
      (return true)
      (else
        (Default|GetServerMessage (LocalVariables|GetLocalPlayerController) "Failed to get character selection.")
        (return false)))
    (else
      (Default|GetServerMessage (LocalVariables|GetLocalPlayerController) "User file doesn't exist.")
      (return false))))

(fn AttemptRegistry
  (params (PlayerController :type Main%20Player%20Controller%20Object%20Reference) (NewName :type String) (NewPassword :type String))
  ;[1 1 1] Check if User Name already exists.
  (LocalVariables|SetLocalPlayerController PlayerController)
  (LocalVariables|SetLocalUserName NewName)
  (LocalVariables|SetLocalPassword NewPassword)
  (bind _fileexists (CallFunction|FindSaveFile "CSV" (LocalVariables|GetLocalUserName)))
  (if _fileexists
    (Development|PrintString "user name already exists.")
    (return false)
    (else
      ;[1 1 1] Check length of name is appropriate.
      (if (Math|Integer|InRange(Integer) (Utilities|String|Len (LocalVariables|GetLocalUserName)) 5 10)
        ;[1 1 1] Check characters in name.
        (for _array_element (Utilities|String|GetCharacterArrayfromString (Class|KismetStringLibrary|ToUpper (LocalVariables|GetLocalUserName)))
          (if (not (Utilities|Array|ContainsItem (LocalVariables|GetLocalArrayToCheckAgainst) _array_element))
            (LocalVariables|SetNameNotAcceptable true)))
        (if (LocalVariables|GetNameNotAcceptable)
          (Default|GetServerMessage (LocalVariables|GetLocalPlayerController) (Utilities|String|Append "Name must be all letters and 5-10 characters long: " (LocalVariables|GetLocalUserName)))
          (return false)
          (else
            ;[1 1 1] Create save file and send to character creation screen.
            (bind _returnvalue (Class|TextFileManager|SaveArrayText (Utilities|String|Append (Utilities|Struct|BreakDirectoryPath (LocalVariables|GetLocalServerDirectory)) "/CSV") (Utilities|String|Append (LocalVariables|GetLocalUserName) ".csv") (Utilities|Array|MakeArray (Variables|Default|GetUserFileArrayHeader) (Utilities|String|Append "0" "," (LocalVariables|GetLocalUserName))) true))
            (if _returnvalue
              (bind _success (CallFunction|GetCharacterSelection (LocalVariables|GetLocalPlayerController) (LocalVariables|GetLocalUserName)))
              (return _success)
              (else
                (Default|GetServerMessage (LocalVariables|GetLocalPlayerController) "Failed to create User file.")
                (return false)))))
        (else
          (Default|GetServerMessage (LocalVariables|GetLocalPlayerController) (Utilities|String|Append "Name must be all letters and 5-10 characters long: " (LocalVariables|GetLocalUserName)))
          (return false))))))

(fn GetCharacterSelection
  (params (PlayerController :type Main%20Player%20Controller%20Object%20Reference) (UserName :type String))
  (if (Utilities|IsValid PlayerController)
    (Development|PrintString (Utilities|String|Append "LocalPlayerControllerRef: " (Utilities|GetDisplayName PlayerController)))
    (LocalVariables|SetLocalPlayerControllerRef PlayerController)
    (bind _output_get (LocalVariables|SetLocalUserName UserName))
    (bind (_path _fileexists) (CallFunction|FindSaveFile "CSV" _output_get))
    (if _fileexists
      (bind (_stringarray _returnvalue) (Class|TextFileManager|LoadArrayText (.path _path)))
      (if _returnvalue
        (bind _output_get_2 (LocalVariables|SetLocalCharacterFileArray _stringarray))
        (bind _parsedarray (CallFunction|ParseCleanArray 1 _output_get_2))
        (Utilities|Array|RemoveIndex _parsedarray)
        (Utilities|Array|RemoveIndex _parsedarray)
        (LocalVariables|SetLocalSlotsArray _parsedarray)
        (bind _returnvalue_2 (Game|SpawnActorfromClass "/Game/Startup/Characters/BP_StartupCharacterViewer.BP_StartupCharacterViewer_C" (Math|Transform|MakeTransform "0, 0, 0") "AlwaysSpawn" (LocalVariables|GetLocalPlayerControllerRef) 0))
        (bind _output_get_3 (LocalVariables|SetLocalStartupCharacterViewerRef _returnvalue_2))
        (if (Utilities|IsValid _output_get_3)
          (bind _returnvalue_3 (Game|SpawnActorfromClass "/Game/Startup/Characters/BP_CreationCharacter.BP_CreationCharacter_C" (Math|Transform|MakeTransform (+ (Transformation|GetWorldLocation (Variables|/Script/Engine.Character|GetMesh (LocalVariables|GetLocalStartupCharacterViewerRef))) "700.000000,50.000000,300.000000") "0,160.000000, 0") "AdjustIfPossibleButAlwaysSpawn" (LocalVariables|GetLocalPlayerControllerRef) (Utilities|Text|ToText(String) (LocalVariables|GetLocalUserName)) 0))
          (if (Utilities|IsValid _returnvalue_3)
            (Variables|Default|SetCreationCharacterRef _returnvalue_3)
            (Development|PrintString (Utilities|String|Append "owner of " (Utilities|GetDisplayName _returnvalue_3) " is " (Utilities|GetDisplayName (Components|GetOwner _returnvalue_3))))
            (Variables|/Game/Startup/MainPlayerController.MainPlayerController_C|SetCreationCharacterRef (LocalVariables|GetLocalPlayerControllerRef) _returnvalue_3)
            (Default|CreateSelectionWidget (LocalVariables|GetLocalPlayerControllerRef) (LocalVariables|GetLocalUserName) (LocalVariables|GetLocalSlotsArray))
            (return true)
            (else
              (Default|GetServerMessage (LocalVariables|GetLocalPlayerControllerRef) "Failed to spawn main character in player login.")
              (return false)))
          (else
            (Default|GetServerMessage (LocalVariables|GetLocalPlayerControllerRef) "Failed to spawn selection character in player login.")
            (return false)))
        (else
          (Default|GetServerMessage (LocalVariables|GetLocalPlayerControllerRef) "Can't find user file in GM_CharacterSelect > LoadCharacterSelection")
          (return false)))
      (else
        (Default|GetServerMessage (LocalVariables|GetLocalPlayerControllerRef) "Unable to find player file.")
        (return false)))
    (else
      (Default|GetServerMessage (LocalVariables|GetLocalPlayerControllerRef) "No playercontroller in LocalPlayerControllerRef (MainGameState > GetCharacterSelection)"))))

(fn AttemptCreateCharacter
  (params (PlayerController :type Main%20Player%20Controller%20Object%20Reference) (UserName :type String) (CharacterName :type String) (IsMale :type Boolean))
  (LocalVariables|SetLocalPlayerControllerRef PlayerController)
  (LocalVariables|SetLocalUserName UserName)
  (LocalVariables|SetLocalCharacterName CharacterName)
  (LocalVariables|SetLocalIsMale IsMale)
  ;[1 1 1] Check if character already exists
  (bind _fileexists (CallFunction|FindSaveFile "Characters" (LocalVariables|GetLocalCharacterName)))
  (if _fileexists
    (Default|GetServerMessage (LocalVariables|GetLocalPlayerControllerRef) "Character name already exists.")
    (return false)
    (else
      ;[1 1 1] Check length of name is acceptable.
      (if (Math|Integer|InRange(Integer) (Utilities|String|Len (LocalVariables|GetLocalCharacterName)) 5 10)
        ;[1 1 1] Check characters in name are acceptable
        (for _array_element (Utilities|String|GetCharacterArrayfromString (Class|KismetStringLibrary|ToUpper (LocalVariables|GetLocalCharacterName)))
          (if (not (Utilities|Array|ContainsItem (LocalVariables|GetLocalArrayToCheckAgainst) _array_element))
            (LocalVariables|SetNameNotAcceptable true)))
        (if (LocalVariables|GetNameNotAcceptable)
          (Default|GetServerMessage (LocalVariables|GetLocalPlayerControllerRef) "Name must be all letter and 5-10 characters long.")
          (return false)
          (else
            ;[1 1 1] Check if User has available character slot.
            (bind _path (CallFunction|FindSaveFile "CSV" (LocalVariables|GetLocalUserName)))
            (bind (_stringarray _returnvalue) (Class|TextFileManager|LoadArrayText (.path _path)))
            (if _returnvalue
              (bind _output_get (LocalVariables|SetLocalPlayerFileArray _stringarray))
              ;[1 1 1] Get first character slot available.
              (if (<= (Utilities|String|Len (Utilities|Array|Get(acopy) _output_get 2)) 0)
                (LocalVariables|SetLocalSlotAvailable 3) ; Slot avilable is index of array item + 1, since first array item is technically a 0.
                ;[1 1 1] Prepare inventory structure - To change start inventory, add the name of the item to the StarterItemNames array.
                (for _array_element_2 (LocalVariables|GetStarterItemNames) :!label _label
                  (bind _returnvalue_2 (Utilities|GetDataTableRow "/Game/Startup/CSV/CSV_ItemDatabase.CSV_ItemDatabase" _array_element_2)
                    (:then
                      (Utilities|Array|Add (LocalVariables|GetStartingItemArray) _returnvalue_2)
                      ;[1 1 1] Setup character information struct - Edit any of these details to designate starting values.
                      (bind _structout (Utilities|Struct|SetmembersinS_PlayerSaves (Utilities|Struct|MakeS_PlayerSaves (Utilities|Text|ToText(String) (LocalVariables|GetLocalCharacterName)) 6e+01 6e+01 1e+02 1e+02 1e+02 1e+02 6e+01 6e+01 1 0 5 (LocalVariables|GetStartingItemArray) (LocalVariables|GetLocalHeadGear) (LocalVariables|GetLocalChestGear) (LocalVariables|GetLocalArmGear) (LocalVariables|GetLocalBottomGear) (LocalVariables|GetLocalFeetGear) (LocalVariables|GetLocalRightHand) (LocalVariables|GetLocalLeftHand) (LocalVariables|GetLocalBagSlot) 6e+02 1e+03 "(\"None\")" "(\"None\")" (LocalVariables|GetLocalCharacterClass))))
                      ;[0.7893 0.3989 1] Create an array from the Character struct in order to prep for save file. There are probably better ways to parse this, but I haven't gotten to it yet.
                      (Utilities|Array|Clear (LocalVariables|GetLocalCharacterStringArray))
                      (Utilities|Array|Add (LocalVariables|GetLocalCharacterStringArray) (LocalVariables|GetLocalHeaderString))
                      (Utilities|Array|Add (LocalVariables|GetLocalCharacterStringArray) (Utilities|String|JoinStringArray (Utilities|Array|MakeArray (Utilities|String|ToString(Text) (.CharacterName (Utilities|Struct|BreakS_PlayerSaves _structout))) (Utilities|String|ToString(Float) (.Health (Utilities|Struct|BreakS_PlayerSaves _structout))) (Utilities|String|ToString(Float) (.MaxHealth (Utilities|Struct|BreakS_PlayerSaves _structout))) (Utilities|String|ToString(Float) (.Hunger (Utilities|Struct|BreakS_PlayerSaves _structout))) (Utilities|String|ToString(Float) (.MaxHunger (Utilities|Struct|BreakS_PlayerSaves _structout))) (Utilities|String|ToString(Float) (.Thirst (Utilities|Struct|BreakS_PlayerSaves _structout))) (Utilities|String|ToString(Float) (.MaxThirst (Utilities|Struct|BreakS_PlayerSaves _structout))) (Utilities|String|ToString(Float) (.Stamina (Utilities|Struct|BreakS_PlayerSaves _structout))) (Utilities|String|ToString(Float) (.MaxStamina (Utilities|Struct|BreakS_PlayerSaves _structout))) (Utilities|String|ToString(Integer) (.Level (Utilities|Struct|BreakS_PlayerSaves _structout))) (Utilities|String|ToString(Integer) (.EXP (Utilities|Struct|BreakS_PlayerSaves _structout))) (Utilities|String|ToString(Integer) (.StatPoints (Utilities|Struct|BreakS_PlayerSaves _structout))) "INV" (CallFunction|GearStructtoString (.itemid (.EquippedHead (Utilities|Struct|BreakS_PlayerSaves _structout))) (Utilities|String|EnumtoString (.itemname (.EquippedHead (Utilities|Struct|BreakS_PlayerSaves _structout)))) (.itemslot (.EquippedHead (Utilities|Struct|BreakS_PlayerSaves _structout)))) (CallFunction|GearStructtoString (.itemid (.EquippedChest (Utilities|Struct|BreakS_PlayerSaves _structout))) (Utilities|String|EnumtoString (.itemname (.EquippedChest (Utilities|Struct|BreakS_PlayerSaves _structout)))) (.itemslot (.EquippedChest (Utilities|Struct|BreakS_PlayerSaves _structout)))) (CallFunction|GearStructtoString (.itemid (.EquippedArms (Utilities|Struct|BreakS_PlayerSaves _structout))) (Utilities|String|EnumtoString (.itemname (.EquippedArms (Utilities|Struct|BreakS_PlayerSaves _structout)))) (.itemslot (.EquippedArms (Utilities|Struct|BreakS_PlayerSaves _structout)))) (CallFunction|GearStructtoString (.itemid (.EquippedBottom (Utilities|Struct|BreakS_PlayerSaves _structout))) (Utilities|String|EnumtoString (.itemname (.EquippedBottom (Utilities|Struct|BreakS_PlayerSaves _structout)))) (.itemslot (.EquippedBottom (Utilities|Struct|BreakS_PlayerSaves _structout)))) (CallFunction|GearStructtoString (.itemid (.EquippedFeet (Utilities|Struct|BreakS_PlayerSaves _structout))) (Utilities|String|EnumtoString (.itemname (.EquippedFeet (Utilities|Struct|BreakS_PlayerSaves _structout)))) (.itemslot (.EquippedFeet (Utilities|Struct|BreakS_PlayerSaves _structout)))) (CallFunction|GearStructtoString (.itemid (.EquippedRightHand (Utilities|Struct|BreakS_PlayerSaves _structout))) (Utilities|String|EnumtoString (.itemname (.EquippedRightHand (Utilities|Struct|BreakS_PlayerSaves _structout)))) (.itemslot (.EquippedRightHand (Utilities|Struct|BreakS_PlayerSaves _structout)))) (CallFunction|GearStructtoString (.itemid (.EquippedLeftHand (Utilities|Struct|BreakS_PlayerSaves _structout))) (Utilities|String|EnumtoString (.itemname (.EquippedLeftHand (Utilities|Struct|BreakS_PlayerSaves _structout)))) (.itemslot (.EquippedLeftHand (Utilities|Struct|BreakS_PlayerSaves _structout)))) (CallFunction|GearStructtoString (.itemid (.EquippedBag (Utilities|Struct|BreakS_PlayerSaves _structout))) (Utilities|String|EnumtoString (.itemname (.EquippedBag (Utilities|Struct|BreakS_PlayerSaves _structout)))) (.itemslot (.EquippedBag (Utilities|Struct|BreakS_PlayerSaves _structout)))) (Utilities|String|ToString(Float) (.CurrentSpeed (Utilities|Struct|BreakS_PlayerSaves _structout))) (Utilities|String|ToString(Float) (.MaxSpeed (Utilities|Struct|BreakS_PlayerSaves _structout))) (Utilities|String|JoinStringArray (.OwnedMounts (Utilities|Struct|BreakS_PlayerSaves _structout)) "-") (Utilities|String|JoinStringArray (.OwnedPets (Utilities|Struct|BreakS_PlayerSaves _structout)) "-") (Utilities|String|EnumtoString (.PlayerClass (Utilities|Struct|BreakS_PlayerSaves _structout))) (Utilities|String|ToString(Integer) (.Strength (Utilities|Struct|BreakS_PlayerSaves _structout))) (Utilities|String|ToString(Integer) (.Agility (Utilities|Struct|BreakS_PlayerSaves _structout))) (Utilities|String|ToString(Integer) (.Constitution (Utilities|Struct|BreakS_PlayerSaves _structout)))) ","))
                      (bind _output_get_2 (LocalVariables|SetLocalCharacterInventoryStruct (.Inventory (Utilities|Struct|BreakS_PlayerSaves _structout))))
                      ;[1 1 1] Create the Character inventory struct, then make an array from it.
                      (Utilities|Array|Clear (LocalVariables|GetLocalInventoryStringArray))
                      (for _array_element_3 _output_get_2
                        (Utilities|Array|Add (LocalVariables|GetLocalInventoryStringArray) (Utilities|String|Append "," (Utilities|String|JoinStringArray (Utilities|Array|MakeArray (Utilities|String|ToString(Integer) (.ItemID (Utilities|Struct|BreakS_ItemDetails _array_element_3))) (.ItemName (Utilities|Struct|BreakS_ItemDetails _array_element_3)) (.ShortDesc (Utilities|Struct|BreakS_ItemDetails _array_element_3)) (.LongDesc (Utilities|Struct|BreakS_ItemDetails _array_element_3)) (Utilities|String|ToString(Boolean) (.Equipped (Utilities|Struct|BreakS_ItemDetails _array_element_3))) (Utilities|String|ToString(Boolean) (.CanBeEquipped (Utilities|Struct|BreakS_ItemDetails _array_element_3))) (.EquipSlot (Utilities|Struct|BreakS_ItemDetails _array_element_3)) (Utilities|String|ToString(Boolean) (.IsWeapon (Utilities|Struct|BreakS_ItemDetails _array_element_3))) (.WeaponType (Utilities|Struct|BreakS_ItemDetails _array_element_3)) (Utilities|String|ToString(Boolean) (.IsArmor (Utilities|Struct|BreakS_ItemDetails _array_element_3))) (.ArmorType (Utilities|Struct|BreakS_ItemDetails _array_element_3)) (CallFunction|StringArraytoString (.DamageType (Utilities|Struct|BreakS_ItemDetails _array_element_3))) (CallFunction|StringArraytoString (.DefenseType (Utilities|Struct|BreakS_ItemDetails _array_element_3))) (CallFunction|StringArraytoString (.DamageBaseRange (Utilities|Struct|BreakS_ItemDetails _array_element_3))) (CallFunction|StringArraytoString (.ArmorBaseRange (Utilities|Struct|BreakS_ItemDetails _array_element_3))) (Utilities|String|ToString(Float) (.Weight (Utilities|Struct|BreakS_ItemDetails _array_element_3))) (Utilities|String|ToString(Float) (.Cost (Utilities|Struct|BreakS_ItemDetails _array_element_3))) (Utilities|String|ToString(Float) (.ItemHealth (Utilities|Struct|BreakS_ItemDetails _array_element_3))) (Utilities|String|ToString(Float) (.ItemMaxHealth (Utilities|Struct|BreakS_ItemDetails _array_element_3)))) ","))))
                      ;[1 1 1] Save the inventory array to CharacterName_Inventory.cvs in Saves/Inventory folder.
                      (bind _returnvalue_3 (Class|TextFileManager|SaveArrayText (Utilities|String|Append (Utilities|Struct|BreakDirectoryPath (LocalVariables|GetLocalServerDirectory)) "/Inventory") (Utilities|String|Append (LocalVariables|GetLocalCharacterName) "_Inventory.csv") (LocalVariables|GetLocalInventoryStringArray) true))
                      (if _returnvalue_3
                        ;[1 1 1] Create the character save file.
                        (bind _returnvalue_4 (Class|TextFileManager|SaveArrayText (Utilities|String|Append (Utilities|Struct|BreakDirectoryPath (LocalVariables|GetLocalServerDirectory)) "/Characters") (Utilities|String|Append (LocalVariables|GetLocalCharacterName) ".csv") (LocalVariables|GetLocalCharacterStringArray) true))
                        (if _returnvalue_4
                          ;[1 1 1] Overwrite Player file with new character added.
                          (bind _path_2 (CallFunction|FindSaveFile "CSV" (LocalVariables|GetLocalUserName)))
                          (bind (_stringarray_2 _returnvalue_5) (Class|TextFileManager|LoadArrayText (.path _path_2)))
                          (if _returnvalue_5
                            (bind _parsedarray (CallFunction|ParseCleanArray 1 _stringarray_2))
                            (Utilities|Array|Add _parsedarray (LocalVariables|GetLocalCharacterName))
                            (bind _returnvalue_6 (Class|TextFileManager|SaveArrayText "CSV" (LocalVariables|GetLocalUserName) (Utilities|Array|MakeArray "Index,Username,Slot1,Slot2,Slot3,Slot4" (CallFunction|StringArraytoString _parsedarray)) true))
                            (if _returnvalue_6
                              (return true)
                              (else
                                (Default|GetServerMessage (LocalVariables|GetLocalPlayerControllerRef) "Unable to add character to player save data.")
                                (return false)))
                            (else
                              (Default|GetServerMessage (LocalVariables|GetLocalPlayerControllerRef) "Unable to find player save data.")
                              (return false)))
                          (else
                            (Default|GetServerMessage (LocalVariables|GetLocalPlayerControllerRef) "Unable to save character data to file.")
                            (return false)))
                        (else
                          (Default|GetServerMessage (LocalVariables|GetLocalPlayerControllerRef) "Unable to save character inventory data to file.")
                          (return false))))))
                (elif (<= (Utilities|String|Len (Utilities|Array|Get(acopy) _output_get 3)) 0)
                  (LocalVariables|SetLocalSlotAvailable 4)
                  (goto _label)
                  (elif (<= (Utilities|String|Len (Utilities|Array|Get(acopy) _output_get 4)) 0)
                    (LocalVariables|SetLocalSlotAvailable 5)
                    (goto _label)
                    (elif (<= (Utilities|String|Len (Utilities|Array|Get(acopy) _output_get 5)) 0)
                      (LocalVariables|SetLocalSlotAvailable 6)
                      (goto _label)))))
              (else
                (Default|GetServerMessage (LocalVariables|GetLocalPlayerControllerRef) "Unable to locate user save data.")
                (return false)))))
        (else
          (Default|GetServerMessage (LocalVariables|GetLocalPlayerControllerRef) "Name must be all letter and 5-10 characters long.")
          (return false))))))

(fn StringArraytoString
  (params (StringArray :type Array%20of%20Strings))
  (return ""))

(fn LoadCharacterIntoGame
  (params (UserName :type String) (CharacterName :type String) (PlayerController :type Main%20Player%20Controller%20Object%20Reference))
  (bind (_out_data _success) (CallFunction|ParsePlayerDataArray CharacterName 1 false))
  (if _success
    (Default|GetServerMessage PlayerController (Utilities|Array|Get(acopy) (Utilities|String|ParseIntoArray _out_data ", " false)))
    (Default|EnterGameWorld PlayerController)
    (return true)
    (else
      (Default|GetServerMessage PlayerController "Unable to locate character data.")
      (return false))))

(fn OnRepMainCharacterRef)